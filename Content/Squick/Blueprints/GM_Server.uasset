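; GM_Server is the server-side GameMode Blueprint that serves as the server's entry point.
; On BeginPlay it runs a common init that spawns an InstanceEventActor at the origin to trigger events in the Game Instance.
; A server init then logs startup and applies game user settings for a fixed-size window with dynamic resolution.
; Tick is unused, and GetModuleName returns an empty string.
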(event `self.ReceiveBeginPlay`
  ;[1 1 1] GameMode 入口
  (`KismetSystemLibrary.PrintString` "Server RUN")
  (`self.CommonInit`)
  (`self.ServerInit`))

(event `GenerateInstanceEventActor`
  ;[0 0.772 1] 生成场景必要Actor用于触发Game Instance中的事件
  (`|SpawnActorFromClass` "/Game/Squick/Blueprints/InstanceEventActor.InstanceEventActor_C" (`KismetMathLibrary.MakeTransform` (0.0 0.0 0.0)) "Undefined" "OverrideRootScale" null null))

(event `ServerInit`
  ;[1 1 1] 服务端初始化
  (`KismetSystemLibrary.PrintString` "GM_Server 服务端初始化" true true (struct :`G` 0.66 :`B` 1.0 :`A` 1.0) 3600.0)
  (bind _returnvalue (`GameUserSettings.GetGameUserSettings`))
  (`GameUserSettings.SetFullscreenMode` _returnvalue "Windowed")
  (`GameUserSettings.SetDynamicResolutionEnabled` _returnvalue true)
  (`GameUserSettings.SetScreenResolution` _returnvalue (make `IntPoint` 1280 720))
  (`GameUserSettings.SetResolutionScaleNormalized` _returnvalue 1.0)
  (`GameUserSettings.ApplySettings` _returnvalue false))

(event `CommonInit`
  (`self.GenerateInstanceEventActor`))

(fn `GetModuleName`
  (returns (ReturnValue :type String))
  (return ""))

(fn `UserConstructionScript`)
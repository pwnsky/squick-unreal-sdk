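; GM_Lobby is the lobby GameMode Blueprint for the Squick game.
; On BeginPlay it casts the game instance to SquickInstance, has it generate a tick event actor, then calls ShowUI, which is empty here.
; CreateMainMenu lazily creates and caches a WB_Lobby widget for the first player controller, adds it to the viewport and returns it, but nothing in this Blueprint calls it.
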(event `self.ReceiveBeginPlay`
  ;[1 1 1] GameMode 入口
  (bind _asg_instance (cast `/Game/Squick/Blueprints/SquickInstance` (`GameplayStatics.GetGameInstance`)))
  (`/Game/Squick/Blueprints/SquickInstance.GenerateTickEventActor` _asg_instance)
  (`self.Show UI`))

(fn `CreateMainMenu`
  (returns (WB_ProMainMenu :type "/Game/Squick/Widget/WB_Lobby Object Reference"))
  (`/Engine/EditorBlueprintResources/StandardMacros.IsValid` (`self.WB_Lobby`)
    (:`Is Valid`
      _)
    (:`Is Not Valid`
      (bind _returnvalue (`|CreateWidget` "/Game/Squick/Widget/WB_Lobby.WB_Lobby_C" (`GameplayStatics.GetPlayerController` 0)))
      (bind _output_get (set `self.WB_Lobby` _returnvalue))))
  (`UserWidget.AddToViewport` _output_get 0)
  (return (`self.WB_Lobby`)))

(fn `Show UI`)

(fn `UserConstructionScript`)
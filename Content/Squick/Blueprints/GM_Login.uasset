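; GM_Login is the login game mode that starts the Squick client and shows the login screen.
; On BeginPlay it casts the game instance to SquickInstance, generates its tick event actor, runs ClientMain, then calls CreateUI, printing a setup warning if the cast fails.
; CreateUI shows the mouse cursor, creates the WB_Login widget only if no valid one exists, and adds it to the viewport.
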(event `self.ReceiveBeginPlay`
  ;[1 1 1] 初始化实例
  (bind _asg_instance (cast `/Game/Squick/Blueprints/SquickInstance` (`GameplayStatics.GetGameInstance`))
    (:`then`
      (`/Game/Squick/Blueprints/SquickInstance.GenerateTickEventActor` _asg_instance)
      (`/Game/Squick/Blueprints/SquickInstance.ClientMain` _asg_instance)
      (`self.CreateUI`))
    (:`CastFailed`
      (`KismetSystemLibrary.PrintString` "Set intance as G_Instance in settings"))))

(fn `CreateUI`
  (returns (Login :type "/Game/Squick/Widget/WB_Login Object Reference"))
  (bind _returnvalue (`GameplayStatics.GetPlayerController` 0))
  (set `PlayerController.bShowMouseCursor` true _returnvalue)
  (`/Engine/EditorBlueprintResources/StandardMacros.IsValid` (`self.WB_Login`)
    (:`Is Valid`
      _)
    (:`Is Not Valid`
      (bind _returnvalue_2 (`|CreateWidget` "/Game/Squick/Widget/WB_Login.WB_Login_C" _returnvalue))
      (bind _output_get (set `self.WB_Login` _returnvalue_2))))
  (`UserWidget.AddToViewport` _output_get 0)
  (return (`self.WB_Login`)))

(fn `UserConstructionScript`)
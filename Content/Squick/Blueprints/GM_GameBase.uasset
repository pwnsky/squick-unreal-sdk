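; Base GameMode for Squick, bound to Lua module GM_GameBase, with stub player join, connect and offline events for Lua or subclasses.
; BeginPlay has SquickInstance spawn its tick-event actor, then branches to server init or a placeholder single-player mode.
; Server init spawns GameInitFinished to notify the PVP Manager server.
; On GUI server platforms, PostLogin can spawn a one-time Viewer at PlayerStart, possessed by player controller 0.
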(event `OnNewPlayerJoin`
  (params (PlayerController :type "PlayerController Object Reference") (Guid :type String) (Character :type Integer) (Name :type String) (Team :type Integer))
  ;[1 1 1] 子类重写
  (bind _returnvalue (`GameplayStatics.GetActorOfClass` "/Script/Engine.PlayerStart")))

(event `self.ReceiveBeginPlay`
  ;[1 1 1] GameMode 入口
  (bind _asg_instance (cast `/Game/Squick/Blueprints/SquickInstance` (`GameplayStatics.GetGameInstance`)))
  (`/Game/Squick/Blueprints/SquickInstance.GenerateTickEventActor` _asg_instance)
  (if (`/Game/Squick/Blueprints/SquickInstance.IsServer` _asg_instance)
    (`self.ServerInit`) ; 服务端初始化
    (else
      (`self.SingalMode`) ; 如果是多人在线，该Client Init不会运行，这里相当于是单机可以刷副本
    )))

(event `OnPlayerJoin`
  (params (guid :type String) (key :type String) (room_id :type String) (account :type String) (PlayerControllerID :type Integer))
  ;[1 1 1] 玩家请求加入
)

(event `OnPlayerOffline`
  (params (PlayerController :type "PlayerController Object Reference"))
  ;[1 1 1] 子类重写
)

(event `ServerViewer`
  ;[1 1 1] 观看者
  (bind _returnvalue (`GameplayStatics.GetActorOfClass` "/Script/Engine.PlayerStart"))
  (bind _returnvalue_2 (`|SpawnActorFromClass` "/Game/Squick/Blueprints/Viewer.Viewer_C" (`self.GetTransform` _returnvalue) "Undefined" "MultiplyWithRoot" null null))
  (`Controller.Possess` (`GameplayStatics.GetPlayerController` 0) _returnvalue_2))

(event `SingalMode`
  ;[1 1 1] 单人客户端初始化
  (bind _returnvalue (`GameplayStatics.GetActorOfClass` "/Script/Engine.PlayerStart"))
  (`KismetSystemLibrary.PrintString` "Single Player"))

(event `ServerInit`
  ;[1 1 1] 服务端加载完成
  (`KismetSystemLibrary.PrintString` "GameMode服务端初始化" true true (struct :`G` 0.66 :`B` 1.0 :`A` 1.0) 3600.0)
  (`|SpawnActorFromClass` "/Game/Squick/Blueprints/Server/GameInitFinished.GameInitFinished_C" (`KismetMathLibrary.MakeTransform` (0.0 0.0 0.0)) "Undefined" "OverrideRootScale" null null) ; 响应给PVP Manager服务器
)

(event `self.K2_PostLogin`
  (params (NewPlayer :type "PlayerController Object Reference"))
  ;[1 1 1] 新玩家连接
  (`self.IsServerGUI`
    (:`True`
      (if (`self.IsOpenServerViewer`)
        (`self.ServerViewer`)
        (`KismetSystemLibrary.PrintString` "Hello")
        (set `self.IsOpenServerViewer` false)))))

(event `OnPlayerConnected`
  (params (player :type "PlayerController Object Reference"))
  ;[1 1 1] 新玩家连接
)

(fn `GetModuleName`
  (returns (ReturnValue :type String))
  (return "GM_GameBase"))

(fn `UserConstructionScript`)